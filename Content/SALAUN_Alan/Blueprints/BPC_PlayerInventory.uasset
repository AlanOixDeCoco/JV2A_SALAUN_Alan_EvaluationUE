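; Player component that tracks health and the count of collected Korogus.
; Health starts at MaxHealth on BeginPlay, and each change to health or count is printed and pushed to BP_MyPlayerController for the UI.
; TakeDamage always removes one point, ignoring its Damage input, and opens EvalTestMap when health reaches zero.
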(event `self.ReceiveBeginPlay`
  (set `self.Health` (`self.MaxHealth`)))

(fn `CollectKorogu`
  (bind _result (`/Engine/EditorBlueprintResources/StandardMacros.IncrementInt` (`self.KoroguCount`))
    (:`  `
      (bind _output_get (set `self.KoroguCount` _result))
      (`KismetSystemLibrary.PrintText` (`KismetTextLibrary.Conv_IntToText` _output_get))
      (bind _asbp_my_player_controller (cast `/Game/SALAUN_Alan/Blueprints/BP_MyPlayerController` (`GameplayStatics.GetPlayerController` 0)))
      (`/Game/SALAUN_Alan/Blueprints/BP_MyPlayerController.SetKorogusCount` _asbp_my_player_controller (`self.KoroguCount`)))))

(fn `TakeDamage`
  (params (Damage :type Integer :default 1))
  (bind _result (`/Engine/EditorBlueprintResources/StandardMacros.DecrementInt` (`self.Health`))
    (:`  `
      (bind _output_get (set `self.Health` _result))
      (`KismetSystemLibrary.PrintText` (`KismetTextLibrary.Conv_IntToText` _output_get))
      (`|ExecutionSequence`
        (:`then_0`
          (bind _asbp_my_player_controller (cast `/Game/SALAUN_Alan/Blueprints/BP_MyPlayerController` (`GameplayStatics.GetPlayerController` 0)))
          (`/Game/SALAUN_Alan/Blueprints/BP_MyPlayerController.SetUIHealth` _asbp_my_player_controller (`self.Health`) (`self.MaxHealth`)))
        (:`then_1`
          (if (<= (`self.Health`) 0)
            (`KismetSystemLibrary.PrintText` "Died from damage!")
            (`GameplayStatics.OpenLevelBySoftObjectPtr` "/Game/SALAUN_Alan/Maps/EvalTestMap.EvalTestMap")))))))